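; Interactable lift that moves its mesh between a start point and an end point.
; Stepping into the lift trigger or interacting sends it to the opposite end, found by comparing mesh position to both points, unless already moving.
; Enabled landing triggers activate interaction to call the lift when it rests at the far end.
; Two timelines lerp the mesh, their lengths scaled by travel distance at BeginPlay, which also debug-prints the duration.
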(event `self.ReceiveBeginPlay`
  (bind _returnvalue (* (* (`KismetMathLibrary.VSize` (- (`SceneComponent.K2_GetComponentLocation` (`self.EndPoint`)) (`SceneComponent.K2_GetComponentLocation` (`self.StartPoint`)))) 0.01) 0.25))
  (`parent.ReceiveBeginPlay`)
  (`TimelineComponent.SetTimelineLength` (`self.TLDoorToStart`) _returnvalue)
  (`TimelineComponent.SetTimelineLength` (`self.TLDoorToEnd`) _returnvalue)
  (`KismetSystemLibrary.PrintString` (`KismetStringLibrary.Conv_DoubleToString` _returnvalue) true true (struct :`G` 0.66 :`B` 1.0 :`A` 1.0) 5.0))

(event `self.ReceiveTick`
  (params (DeltaSeconds :type "Float (single-precision)"))
  (`parent.ReceiveTick` DeltaSeconds))

(event `self.liftTrigger.OnComponentBeginOverlap`
  (params (OverlappedComponent :type "PrimitiveComponent Object Reference") (OtherActor :type "Actor Object Reference") (OtherComp :type "PrimitiveComponent Object Reference") (OtherBodyIndex :type Integer) (bFromSweep :type Boolean) (SweepResult :type "HitResult Structure (by ref)"))
  (if (not (`self.isMoving`))
    (`self.Move`)))

(event `self.StartTrigger.OnComponentBeginOverlap`
  (params (OverlappedComponent :type "PrimitiveComponent Object Reference") (OtherActor :type "Actor Object Reference") (OtherComp :type "PrimitiveComponent Object Reference") (OtherBodyIndex :type Integer) (bFromSweep :type Boolean) (SweepResult :type "HitResult Structure (by ref)"))
  (bind (_start _end) (`self.GetLiftPos`))
  (if (and _end (`self.startEnabled`) (not (`self.isMoving`)))
    (`self.ActivateInteractable` OtherActor)))

(event `self.StartTrigger.OnComponentEndOverlap`
  (params (OverlappedComponent :type "PrimitiveComponent Object Reference") (OtherActor :type "Actor Object Reference") (OtherComp :type "PrimitiveComponent Object Reference") (OtherBodyIndex :type Integer))
  (`self.DeactivateIneractable` OtherActor))

(event `self.EndTrigger.OnComponentBeginOverlap`
  (params (OverlappedComponent :type "PrimitiveComponent Object Reference") (OtherActor :type "Actor Object Reference") (OtherComp :type "PrimitiveComponent Object Reference") (OtherBodyIndex :type Integer) (bFromSweep :type Boolean) (SweepResult :type "HitResult Structure (by ref)"))
  (bind _start (`self.GetLiftPos`))
  (if (and _start (`self.endEnabled`) (not (`self.isMoving`)))
    (`self.ActivateInteractable` OtherActor)))

(event `self.EndTrigger.OnComponentEndOverlap`
  (params (OverlappedComponent :type "PrimitiveComponent Object Reference") (OtherActor :type "Actor Object Reference") (OtherComp :type "PrimitiveComponent Object Reference") (OtherBodyIndex :type Integer))
  (`self.DeactivateIneractable` OtherActor))

(event `Move`
  (set `self.isMoving` true)
  (bind (_start _end) (`self.GetLiftPos`))
  (if _start
    (`self.MoveToEnd`)
    (elif _end
      (`self.MoveToStart`))))

(event `MoveToStart`
  (set `self.isMoving` true)
  (bind (_direction _newtrack_0) (`Timeline|TLDoorToStart` :!via `PlayFromStart`)
    (:`Update`
      (`SceneComponent.K2_SetWorldLocation` (`self.StaticMesh`) (`KismetMathLibrary.VLerp` (`SceneComponent.K2_GetComponentLocation` (`self.EndPoint`)) (`SceneComponent.K2_GetComponentLocation` (`self.StartPoint`)) _newtrack_0) false false))
    (:`Finished`
      (set `self.isMoving` false))))

(event `MoveToEnd`
  (set `self.isMoving` true)
  (bind (_direction _newtrack_0) (`Timeline|TLDoorToEnd` :!via `PlayFromStart`)
    (:`Update`
      (`SceneComponent.K2_SetWorldLocation` (`self.StaticMesh`) (`KismetMathLibrary.VLerp` (`SceneComponent.K2_GetComponentLocation` (`self.StartPoint`)) (`SceneComponent.K2_GetComponentLocation` (`self.EndPoint`)) _newtrack_0) false false))
    (:`Finished`
      (set `self.isMoving` false))))

(fn `GetLiftPos`
  (returns (Start :type Boolean) (End :type Boolean))
  (if (== (`SceneComponent.K2_GetComponentLocation` (`self.StaticMesh`)) (`SceneComponent.K2_GetComponentLocation` (`self.StartPoint`)) :`ErrorTolerance` 0.001)
    (return true false)
    (elif (== (`SceneComponent.K2_GetComponentLocation` (`self.StaticMesh`)) (`SceneComponent.K2_GetComponentLocation` (`self.EndPoint`)) :`ErrorTolerance` 0.001)
      (return false true)
      (else
        (return false false)))))

(fn `Interact`
  (`parent.Interact`)
  (if (not (`self.isMoving`))
    (`self.Move`)))

(fn `LerpVectors`
  (params (Start :type "Vector Structure") (End :type "Vector Structure") (Alpha :type "Float (double-precision)")))

(fn `UserConstructionScript`
  (`parent.UserConstructionScript`))