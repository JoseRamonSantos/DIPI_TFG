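; Interactable door that swings open when used and persists its opened state through MyGameInstance.
; Front and back trigger boxes, each with an enable flag, feed the parent's activate and deactivate interaction logic.
; Interacting runs a timeline that lerps mesh yaw toward OpenAngle, then clears Activated and saves it.
; BeginPlay registers the door by display name plus level name and can snap it open from saved state.
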(event `self.ReceiveBeginPlay`
  (`parent.ReceiveBeginPlay`)
  (bind _asmy_game_instance (cast `/Game/BPs/MyGameInstance` (`GameplayStatics.GetGameInstance`)))
  (bind _name (`self.GetName`))
  (bind _exist_ (`/Game/BPs/MyGameInstance.AddDoorData` _asmy_game_instance (make `/Game/BPs/Interactable/S_DoorData` _name (`self.activated`))))
  (if _exist_
    (bind _name_2 (`self.GetName`))
    (bind _data (`/Game/BPs/MyGameInstance.GetSavedDoorData` _asmy_game_instance (make `/Game/BPs/Interactable/S_DoorData` _name_2)))
    (bind _output_get (set `self.activated` (`.activated_5_D6AD9A4C4B3C8A03DC1B5FA59BF73A7B` (break `/Game/BPs/Interactable/S_DoorData` _data))))
    (if (not _output_get)
      (`self.OpenDoorInstant`))))

(event `self.FrontBox.OnComponentBeginOverlap`
  (params (OverlappedComponent :type "PrimitiveComponent Object Reference") (OtherActor :type "Actor Object Reference") (OtherComp :type "PrimitiveComponent Object Reference") (OtherBodyIndex :type Integer) (bFromSweep :type Boolean) (SweepResult :type "HitResult Structure (by ref)"))
  (if (`self.frontOpenEnabled`)
    (`self.ActivateInteractable` OtherActor)))

(event `self.FrontBox.OnComponentEndOverlap`
  (params (OverlappedComponent :type "PrimitiveComponent Object Reference") (OtherActor :type "Actor Object Reference") (OtherComp :type "PrimitiveComponent Object Reference") (OtherBodyIndex :type Integer))
  (if (`self.frontOpenEnabled`)
    (`self.DeactivateIneractable` OtherActor)))

(event `self.BackBox.OnComponentBeginOverlap`
  (params (OverlappedComponent :type "PrimitiveComponent Object Reference") (OtherActor :type "Actor Object Reference") (OtherComp :type "PrimitiveComponent Object Reference") (OtherBodyIndex :type Integer) (bFromSweep :type Boolean) (SweepResult :type "HitResult Structure (by ref)"))
  (if (`self.backOpenEnabled`)
    (`self.ActivateInteractable` OtherActor)))

(event `self.BackBox.OnComponentEndOverlap`
  (params (OverlappedComponent :type "PrimitiveComponent Object Reference") (OtherActor :type "Actor Object Reference") (OtherComp :type "PrimitiveComponent Object Reference") (OtherBodyIndex :type Integer))
  (if (`self.backOpenEnabled`)
    (`self.DeactivateIneractable` OtherActor)))

(event `OpenDoor`
  (bind (_direction _newtrack_0) (`Timeline|Timeline_0`)
    (:`Update`
      (bind (_crntrotation _desiredrotation) (`self.GetRotations`))
      (`SceneComponent.K2_SetRelativeRotation` (`self.StaticMesh`) (`KismetMathLibrary.RLerp` _crntrotation _desiredrotation _newtrack_0 true) false false))))

(event `OpenDoorInstant`
  (bind (_crntrotation _desiredrotation) (`self.GetRotations`))
  (`SceneComponent.K2_SetRelativeRotation` (`self.StaticMesh`) _desiredrotation false false))

(event `UpdateData`
  (bind _asmy_game_instance (cast `/Game/BPs/MyGameInstance` (`GameplayStatics.GetGameInstance`)))
  (bind _name (`self.GetName`))
  (`/Game/BPs/MyGameInstance.UpdateDoorData` _asmy_game_instance (make `/Game/BPs/Interactable/S_DoorData` _name (`self.activated`))))

(fn `ActivateInteractable`
  (params (player :type "Actor Object Reference"))
  (`parent.ActivateInteractable` player))

(fn `GetName`
  (returns (name :type String))
  (bind _returnvalue (`GameplayStatics.GetCurrentLevelName` true))
  (return (`KismetStringLibrary.Concat_StrStr` (`KismetSystemLibrary.GetDisplayName` self) "_" _returnvalue)))

(fn `GetRotations`
  (returns (crntRotation :type "Rotator Structure") (desiredRotation :type "Rotator Structure"))
  (bind _staticmesh (`self.StaticMesh`))
  (bind (_relativerotation_roll _relativerotation_pitch) (`KismetMathLibrary.BreakRotator` (`SceneComponent.RelativeRotation` _staticmesh)))
  (return (`SceneComponent.RelativeRotation` _staticmesh) (`KismetMathLibrary.MakeRotator` _relativerotation_roll _relativerotation_pitch (`self.openAngle`))))

(fn `Interact`
  (`parent.Interact`)
  (`self.OpenDoor`)
  (set `self.activated` false)
  (`self.UpdateData`))

(fn `UserConstructionScript`
  (`parent.UserConstructionScript`))