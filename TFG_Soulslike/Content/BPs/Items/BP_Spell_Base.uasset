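; Base spell actor that damages characters overlapping its scalable sphere, skipping the instigator and invulnerable characters.
; CalculateHit passes targets to DoDamage and records them in HitChars, which ResetHitChar clears per character after an optional delay.
; Its already-hit check fires per differing list entry, so hits can repeat.
; Beyond a maximum distance, DoDamage decays and overwrites the stored Damage, then applies the attack modifier, printing debug text.
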(event `self.ReceiveBeginPlay`
  (`parent.ReceiveBeginPlay`))

(event `ResetHitChar`
  (params (char :type "/Game/BPs/Char/BP_Char_Base Object Reference"))
  (if (!= (`self.resetHitTime`) 0.0)
    (`KismetSystemLibrary.Delay` (`self.resetHitTime`))
    (`KismetArrayLibrary.Array_RemoveItem` (`self.hitChars`) char)))

(fn `CalculateHit`
  (bind (_arrayindex _arrayelement) (`/Engine/EditorBlueprintResources/StandardMacros.ReverseForEachLoop` (`PrimitiveComponent.GetOverlappingActors` (`self.Sphere`) "/Game/BPs/Char/BP_Char_Base.BP_Char_Base_C"))
    (:`LoopBody`
      (if (!= _arrayelement (`self.Instigator`))
        (if (> (`KismetArrayLibrary.Array_Length` (`self.hitChars`)) 0)
          (bind (_arrayindex_2 _arrayelement_2) (`/Engine/EditorBlueprintResources/StandardMacros.ReverseForEachLoop` (`self.hitChars`))
            (:`LoopBody`
              (if (!= _arrayelement_2 _arrayelement)
                (bind _asbp_char_base (cast `/Game/BPs/Char/BP_Char_Base` _arrayelement :!label _label))
                (if (not (`/Game/BPs/Char/BP_Char_Base.isInvulnerable` _asbp_char_base))
                  (`self.DoDamage` _asbp_char_base)
                  (`KismetArrayLibrary.Array_Add` (`self.hitChars`) _asbp_char_base)))))
          (else
            (goto _label)))))))

(fn `DoDamage`
  (params (targetToDamage :type "/Game/BPs/Char/BP_Char_Base Object Reference"))
  (bind (_attackinfo_attack _attackinfo_staminacost _attackinfo_anim _attackinfo_damagemodifier) (break `/Game/BPs/Char/S_CharAttackInfo` (`self.attackInfo`)))
  (bind _maxdamagedistance (`self.maxDamageDistance`))
  (bind _damage (`self.damage`))
  (bind _returnvalue (`KismetMathLibrary.Vector_Distance` (`self.K2_GetActorLocation` targetToDamage) (`self.K2_GetActorLocation` self)))
  (bind _returnvalue_2 (- _returnvalue _maxdamagedistance))
  (bind _returnvalue_3 (* _returnvalue_2 (`self.damageDecay`)))
  (bind _returnvalue_4 (* _damage _returnvalue_3))
  (bind _returnvalue_5 (`KismetMathLibrary.FClamp` (- _damage _returnvalue_4) 0.0 (`KismetMathLibrary.Abs` _damage)))
  (if (not (== (`self.maxDamageDistance`) 0.0))
    (`KismetSystemLibrary.PrintString` (`KismetStringLibrary.Concat_StrStr` "Max Distance: " (`KismetStringLibrary.Conv_DoubleToString` _maxdamagedistance) "Distance: " (`KismetStringLibrary.Conv_DoubleToString` _returnvalue)) true true (struct :`G` 0.364575 :`B` 0.755208 :`A` 1.0) 20.0)
    (if (not (<= _returnvalue _maxdamagedistance))
      (`KismetSystemLibrary.PrintString` (`KismetStringLibrary.Concat_StrStr` "  Distance: " (`KismetStringLibrary.Conv_DoubleToString` _returnvalue_2) "  Damage Reduction Percent: " (`KismetStringLibrary.Conv_DoubleToString` _returnvalue_3) "  ( " (`KismetStringLibrary.Conv_DoubleToString` _returnvalue_4) ")  //Damage: " (`KismetStringLibrary.Conv_DoubleToString` _damage) "  --> " (`KismetStringLibrary.Conv_DoubleToString` _returnvalue_5)) true true (struct :`R` 0.755208 :`G` 0.541201 :`A` 1.0) 20.0)
      (set `self.damage` _returnvalue_5)))
  (`/Game/BPs/Char/BP_Char_Base.TakeDamage` targetToDamage (`self.attackInfo`) (* (`self.damage`) _attackinfo_damagemodifier) 1.0)
  (`self.ResetHitChar` targetToDamage)
  (`KismetSystemLibrary.PrintString` (`KismetStringLibrary.Concat_StrStr` (`KismetSystemLibrary.GetDisplayName` self) " DO DAMAGE TO: " (`KismetSystemLibrary.GetDisplayName` targetToDamage)) true true (struct :`R` 1.0 :`B` 0.1 :`A` 1.0)))

(fn `ModifyScaleUniform`
  (params (Value :type "Float (double-precision)"))
  (`SceneComponent.SetWorldScale3D` (`self.Sphere`) (* (1.0 1.0 1.0) Value)))

(fn `UserConstructionScript`
  (`parent.UserConstructionScript`))