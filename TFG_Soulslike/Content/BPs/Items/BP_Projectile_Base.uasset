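; Base projectile actor that deals damage to characters on impact.
; On a sphere component hit it ignores its instigator and other projectiles, and passes its attack info and damage to any BP_Char_Base it strikes.
; Any other valid hit, character or not, spawns a scaled impact particle and destroys the projectile.
; Each hit also prints the struck actor's name as debug output.
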(event `self.Sphere.OnComponentHit`
  (params (HitComponent :type "PrimitiveComponent Object Reference") (OtherActor :type "Actor Object Reference") (OtherComp :type "PrimitiveComponent Object Reference") (NormalImpulse :type "Vector Structure") (Hit :type "HitResult Structure (by ref)"))
  (bind (_returnvalue_location _returnvalue_rotation) (`KismetMathLibrary.BreakTransform` (`self.GetTransform`)))
  (`KismetSystemLibrary.PrintString` (`KismetSystemLibrary.GetDisplayName` OtherActor))
  (if (!= OtherActor (`self.Instigator`))
    (cast `/Game/BPs/Items/BP_Projectile_Base` OtherActor
      (:`CastFailed`
        (bind _asbp_char_base (cast `/Game/BPs/Char/BP_Char_Base` OtherActor)
          (:`then`
            (`/Game/BPs/Char/BP_Char_Base.TakeDamage` _asbp_char_base (`self.attackInfo`) (* (`self.damage`) 1.0) 1.0))
          (:`CastFailed`
            _))
        (`GameplayStatics.SpawnEmitterAtLocation` (`self.impactParticle`) _returnvalue_location _returnvalue_rotation (* (1.0 1.0 1.0) (`self.impactParticlesScale`)))
        (`self.K2_DestroyActor`)))))

(fn `UserConstructionScript`)