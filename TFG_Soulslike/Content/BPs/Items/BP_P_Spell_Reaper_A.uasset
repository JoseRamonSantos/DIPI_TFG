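; Reaper spell item actor that repeatedly applies hit checks while it scales over its lifetime.
; On BeginPlay it runs the parent logic, then starts a fast looping timer that calls CalculateHit and a one-shot timer set to Duration.
; A timeline drives ModifyScaleUniform to animate its size.
; When the duration elapses, it clears both timers and destroys itself.
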(event `self.ReceiveBeginPlay`
  (`parent.ReceiveBeginPlay`)
  (bind _returnvalue (`KismetSystemLibrary.K2_SetTimerDelegate` (delegate `HIt`) 0.05 true))
  (bind _returnvalue_2 (`KismetSystemLibrary.K2_SetTimerDelegate` (delegate `Destroy`) (`self.duration`)))
  (bind (_direction _newtrack_0) (`Timeline|Timeline_0` :!via `PlayFromStart`)
    (:`Update`
      (`self.ModifyScaleUniform` _newtrack_0))))

(event `HIt`
  (`self.CalculateHit`))

(event `Destroy`
  (`KismetSystemLibrary.K2_ClearAndInvalidateTimerHandle` (stale `self.ReceiveBeginPlay` _returnvalue))
  (`KismetSystemLibrary.K2_ClearAndInvalidateTimerHandle` (stale `self.ReceiveBeginPlay` _returnvalue_2))
  (`self.K2_DestroyActor`))

(fn `UserConstructionScript`
  (`parent.UserConstructionScript`))