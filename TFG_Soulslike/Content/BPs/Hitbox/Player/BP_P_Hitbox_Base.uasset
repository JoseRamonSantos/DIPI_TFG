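; Base Blueprint for player hitboxes that applies weapon damage to enemies.
; DoDamage extends the parent function by looping over BP_Enemy_Base actors overlapping the hitbox, with BP_Player as instigator.
; The Item hand selects the player's right or left current weapon, whose damage is scaled by DamageModifier and sent with HitStrength to each enemy's ReceiveDamage.
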(fn `DoDamage`
  (bind _overlappingactors (`PrimitiveComponent.GetOverlappingActors` (`self.Hitbox`) "/Game/BPs/Char/Enemies/BP_Enemy_Base.BP_Enemy_Base_C"))
  (`parent.DoDamage`)
  (for _index (range (+ (`KismetArrayLibrary.Array_Length` _overlappingactors) 1))
    (bind _asbp_enemy_base (cast `/Game/BPs/Char/Enemies/BP_Enemy_Base` (`|GetArrayItem` _overlappingactors _index)))
    (set `self.target` _asbp_enemy_base)
    (bind _asbp_player (cast `/Game/BPs/Char/Player/BP_Player` (`self.Instigator`)))
    (switch `/Game/BPs/Items/E_ItemHand` (`self.item`)
      (:`NewEnumerator0`
        (bind _crntweapon1 (`/Game/BPs/Char/Player/BP_Player.crntWeapon1` _asbp_player))
        (`/Engine/EditorBlueprintResources/StandardMacros.IsValid` _crntweapon1
          (:`Is Valid`
            (bind _damage (`/Game/BPs/Items/BP_Item_Weapon.GetDamage` _crntweapon1))
            (set `self.finalDamage` (* _damage (`self.damageModifier`))))))
      (:`NewEnumerator1`
        (bind _crntweapon2 (`/Game/BPs/Char/Player/BP_Player.crntWeapon2` _asbp_player))
        (`/Engine/EditorBlueprintResources/StandardMacros.IsValid` _crntweapon2
          (:`Is Valid`
            (bind _damage_2 (`/Game/BPs/Items/BP_Item_Weapon.GetDamage` _crntweapon2))
            (set `self.finalDamage` (* _damage_2 (`self.damageModifier`)))))))
    (`/Game/BPs/Char/BP_Char_Base.ReceiveDamage` (`self.target`) (`self.finalDamage`) (`self.hitStrength`))))

(fn `UserConstructionScript`
  (`parent.UserConstructionScript`))