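; Base hitbox Blueprint for enemy attacks that applies damage to players overlapping it.
; Its DoDamage override calls the parent, then loops over BP_Player actors inside the Hitbox.
; Each player receives the instigating BP_Enemy_Base's damage scaled by DamageModifier, along with a HitStrength value.
; The event graph holds only disabled stubs, so this asset adds no overlap or tick logic.
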(fn `DoDamage`
  (bind _overlappingactors (`PrimitiveComponent.GetOverlappingActors` (`self.Hitbox`) "/Game/BPs/Char/Player/BP_Player.BP_Player_C"))
  (`parent.DoDamage`)
  (for _index (range (+ (`KismetArrayLibrary.Array_Length` _overlappingactors) 1))
    (bind _asbp_player (cast `/Game/BPs/Char/Player/BP_Player` (`|GetArrayItem` _overlappingactors _index)))
    (set `self.target` _asbp_player)
    (bind _asbp_enemy_base (cast `/Game/BPs/Char/Enemies/BP_Enemy_Base` (`self.Instigator`)))
    (bind _basedamage (`/Game/BPs/Char/Enemies/BP_Enemy_Base.GetDamage` _asbp_enemy_base))
    (set `self.finalDamage` (* _basedamage (`self.damageModifier`)))
    (`/Game/BPs/Char/BP_Char_Base.ReceiveDamage` (`self.target`) (`self.finalDamage`) (`self.hitStrength`))))

(fn `UserConstructionScript`
  (`parent.UserConstructionScript`))