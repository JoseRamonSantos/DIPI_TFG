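; Basic skeleton archer enemy Blueprint that supplies the transform for shooting from its bow toward the player.
; GetShootPos starts at the Bow's world location and aims X at the player mesh's targetSocket via MakeRotFromXZ.
; The rotation's Z reference is the bow's world location rather than an up vector, so roll varies with position.
; The construction script only calls the parent, and the event graph holds just disabled stubs.
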(fn `GetShootPos`
  (returns (shootPos :type "Transform Structure"))
  (bind _returnvalue_location (`KismetMathLibrary.BreakTransform` (`SceneComponent.K2_GetComponentToWorld` (`self.Bow`))))
  (bind _asbp_player (cast `/Game/BPs/Char/Player/BP_Player` (`GameplayStatics.GetPlayerPawn` 0)))
  (bind _returnvalue_location_2 (`KismetMathLibrary.BreakTransform` (`SceneComponent.GetSocketTransform` (`Character.Mesh` _asbp_player) "targetSocket" "RTS_World")))
  (return (`KismetMathLibrary.MakeTransform` _returnvalue_location (`KismetMathLibrary.MakeRotFromXZ` (- _returnvalue_location_2 _returnvalue_location) _returnvalue_location))))

(fn `UserConstructionScript`
  (`parent.UserConstructionScript`))