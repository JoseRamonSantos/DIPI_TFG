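; BP_BE_Corspe is the Corpse variant of the basic enemy, inheriting its core behavior from a parent class.
; It overrides ChangeState to call the parent, then set a distinct move type for each of the Patrol, Chase and Attack states.
; It also supplies hitbox start and end positions from the world locations of its StartHitbox and EndHitbox components.
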(event `self.ReceiveBeginPlay`
  (`parent.ReceiveBeginPlay`))

(fn `ChangeState`
  (params (newState :type "/Game/BPs/Char/Enemies/BasicEnemy/e_basicEnemyStates Enum" :default "NewEnumerator0"))
  (`parent.ChangeState` newState)
  (switch `/Game/BPs/Char/Enemies/BasicEnemy/e_basicEnemyStates` newState
    (:`NewEnumerator0`
      (`self.ChangeMoveType` "NewEnumerator0"))
    (:`NewEnumerator1`
      (`self.ChangeMoveType` "NewEnumerator2"))
    (:`NewEnumerator2`
      (`self.ChangeMoveType` "NewEnumerator1"))))

(fn `GetStartAndEndHitboxPos`
  (returns (start :type "Vector Structure") (end :type "Vector Structure"))
  (return (`SceneComponent.K2_GetComponentLocation` (`self.startHitbox`)) (`SceneComponent.K2_GetComponentLocation` (`self.endHitbox`))))

(fn `UserConstructionScript`
  (`parent.UserConstructionScript`))