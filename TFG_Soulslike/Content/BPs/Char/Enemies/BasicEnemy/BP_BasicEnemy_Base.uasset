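; Base Blueprint for basic enemies that manages the enemy's HP bar widget.
; InitHUD casts the HPBar component's widget to UI_EnemyHPBar, caches it and initializes it from the passed stats.
; DecreaseHPBar forwards stats to the cached widget, printing an error if it is unassigned, and two events show or hide the bar.
; BeginPlay and construction only call the parent class.
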(event `self.ReceiveBeginPlay`
  (`parent.ReceiveBeginPlay`))

(event `HideHPBar`
  (`SceneComponent.SetVisibility` (`self.HPBar`) false false))

(event `ShowHPBar`
  (`SceneComponent.SetVisibility` (`self.HPBar`) true false))

(fn `DecreaseHPBar`
  (params (stats :type "/Game/BPs/Char/S_CharStats Structure"))
  (if (`KismetSystemLibrary.IsValid` (`self.widgetHPBar`))
    (`/Game/UI/UI_EnemyHPBar.DecreaseHP` (`self.widgetHPBar`) (`local.stats`))
    (else
      (`KismetSystemLibrary.PrintString` "Unasigned EnemyHPBar. Enemy: DecreaseHPBar" true true (struct :`R` 1.0 :`A` 1.0) 5.0)))
  (return))

(fn `InitHUD`
  (params (Stats :type "/Game/BPs/Char/S_CharStats Structure"))
  (bind _asui_enemy_hpbar (cast `/Game/UI/UI_EnemyHPBar` (`WidgetComponent.GetUserWidgetObject` (`self.HPBar`))))
  (bind _output_get (set `self.widgetHPBar` _asui_enemy_hpbar))
  (`/Game/UI/UI_EnemyHPBar.InitValues` _output_get (`local.Stats`)))

(fn `UserConstructionScript`
  (`parent.UserConstructionScript`))