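; Normal Barghest variant of the basic enemy, a child Blueprint that extends its parent's setup and state handling.
; On BeginPlay the mane and tail meshes follow the main Mesh through master pose.
; ChangeState maps Patrol, Chase and Attack to move types, and two arrow components supply the hitbox start and end positions.
; Capsule hits on the player only print a debug message.
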(event `self.ReceiveBeginPlay`
  (`parent.ReceiveBeginPlay`)
  (`SkinnedMeshComponent.SetLeaderPoseComponent` (`self.SK_BARGHEST_MANE`) (`self.Mesh`) false)
  (`SkinnedMeshComponent.SetLeaderPoseComponent` (`self.SK_BARGHEST_TAIL`) (`self.Mesh`) false))

(event `self.Capsule.OnComponentHit`
  (params (HitComponent :type "PrimitiveComponent Object Reference") (OtherActor :type "Actor Object Reference") (OtherComp :type "PrimitiveComponent Object Reference") (NormalImpulse :type "Vector Structure") (Hit :type "HitResult Structure (by ref)"))
  (cast `/Game/BPs/Char/Player/BP_Player` OtherActor)
  (`KismetSystemLibrary.PrintString` "HIT PLAYER"))

(fn `ChangeState`
  (params (newState :type "/Game/BPs/Char/Enemies/BasicEnemy/e_basicEnemyStates Enum" :default "NewEnumerator0"))
  (`parent.ChangeState` newState)
  (switch `/Game/BPs/Char/Enemies/BasicEnemy/e_basicEnemyStates` newState
    (:`NewEnumerator0`
      (`self.ChangeMoveType` "NewEnumerator0"))
    (:`NewEnumerator1`
      (`self.ChangeMoveType` "NewEnumerator2"))
    (:`NewEnumerator2`
      (`self.ChangeMoveType` "NewEnumerator1"))))

(fn `GetStartAndEndHitboxPos`
  (returns (start :type "Vector Structure") (end :type "Vector Structure"))
  (return (`SceneComponent.K2_GetComponentLocation` (`self.Arrow1`)) (`SceneComponent.K2_GetComponentLocation` (`self.Arrow2`))))

(fn `UserConstructionScript`
  (`parent.UserConstructionScript`))